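; Projectile Blueprint that plays a shotgun blast sound when it spawns.
; The construction script assigns the launch and impact particle templates and sets an invisible sphere as the collision mesh.
; BeginPlay plays the attenuated shot sound at the launch blast component's location.
; Movement and impact handling are not scripted in these graphs.
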(event EventBeginPlay
  ;[1 1 1] PlayShootingSfx
  (Audio|PlaySoundatLocation "/Game/Sound/Shotgun_Blast-Jim_Rogers-1914772763.Shotgun_Blast-Jim_Rogers-1914772763" (Transformation|GetWorldLocation (Variables|Default|GetLaunchBlast)) "0, 0, 0" 1.0 1.0 0.0 "/Game/Sound/ShootingAttenuation.ShootingAttenuation" 0 0))

(fn ConstructionScript
  (bind _collisionmesh (Variables|Default|GetCollisionMesh))
  (Effects|Components|ParticleSystem|SetTemplate (Variables|Default|GetImpactBlast) "/Game/Projectile/ImpactBlast.ImpactBlast")
  (Effects|Components|ParticleSystem|SetTemplate (Variables|Default|GetLaunchBlast) "/Game/Projectile/LaunchBlast.LaunchBlast")
  (Components|StaticMesh|SetStaticMesh _collisionmesh "/Game/Projectile/Shape_Sphere.Shape_Sphere")
  (Rendering|SetVisibility _collisionmesh false false))