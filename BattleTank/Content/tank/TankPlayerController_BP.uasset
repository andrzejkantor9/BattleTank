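; Tank player controller Blueprint that manages the in-game HUD and the game over screen.
; On BeginPlay it creates the PlayerUI widget, adding it to the viewport only after FoundAimingComponent passes it the aiming component reference.
; RemoveUI swaps that HUD for a GameOver widget, shows the mouse cursor and switches input to UI-only.
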(event EventBeginPlay
  ;[1 1 1] Create InGame UI
  (bind _returnvalue (UserInterface|CreateWidget "/Game/UI/PlayerUI.PlayerUI_C"))
  (Variables|Default|SetPlayerUIVariable _returnvalue))

(event EventFoundAimingComponent
  (params (AimCompRef :type Tank%20Aiming%20Component%20Object%20Reference))
  (bind _playeruivariable (Variables|Default|GetPlayerUIVariable))
  ;[1 1 1] Get Reference to Aiming Component for UI
  (Variables|/Game/UI/PlayerUI.PlayerUI_C|SetBP%20AimPoint%20comp%20reference _playeruivariable AimCompRef)
  (UserInterface|Viewport|AddtoViewport _playeruivariable 0))

(fn ConstructionScript)

(fn RemoveUI
  ;[1 1 1] Remove InGame UI
  (Widget|RemovefromParent (Variables|Default|GetPlayerUIVariable))
  ;[1 1 1] Create Game Over UI
  (bind _returnvalue (UserInterface|CreateWidget "/Game/UI/GameOver.GameOver_C"))
  (bind _output_get (Variables|Default|SetGameOverUI _returnvalue))
  (UserInterface|Viewport|AddtoViewport _output_get 0)
  (Variables|Default|SetbShowMouseCursor true)
  (Input|SetInputModeUIOnly (Game|GetPlayerController 0) (Variables|Default|GetGameOverUI) "DoNotLock"))