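; Player-controllable tank pawn Blueprint that routes input to native-style movement and aiming components.
; BeginPlay hands the track meshes to TankMovement and the barrel and turret to TankAiming.
; Axis inputs drive forward and turn intents or rotate the azimuth gimbal and spring arm for camera aim, while Fire calls TankAiming.
; The construction script assigns the turret, barrel and track meshes and enables rigid-body hit notifications on the tracks.
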(event EventBeginPlay
  (Class|TankMovementComponent|InitializeComponent (Variables|Default|GetTankMovement) (Variables|Default|GetTankTrackLeft) (Variables|Default|GetTankTrackRight))
  (Class|TankAimingComponent|InitializeComponent (Variables|Default|GetTankAiming) (Variables|Default|GetBarrel) (Variables|Default|Getturret)))

(event Input|ActionEvents|InputActionFire
  (params (Key :type Key%20Structure))
  ;[1 1 1] Firing projectile
  (:Pressed
    (Class|TankAimingComponent|Fire (Variables|Default|GetTankAiming))))

(event Input|AxisEvents|InputAxisAimAzimuth
  (params (AxisValue :type Float%20%28single-precision%29))
  ;[1 1 1] camera input binding
  (Transformation|AddLocalRotation (Variables|Default|GetAzimuthGimbal) (Math|Rotator|MakeRotator 0.0 0.0 (* AxisValue 0.75)) false false))

(event Input|AxisEvents|InputAxisAimElevation
  (params (AxisValue :type Float%20%28single-precision%29))
  ;[1 1 1] camera input binding
  (Transformation|AddLocalRotation (Variables|Default|GetSpringArm) (Math|Rotator|MakeRotator 0.0 (* AxisValue 0.75) 0.0) false false))

(event Input|AxisEvents|InputAxisTurnRight
  (params (AxisValue :type Float%20%28single-precision%29))
  ;[1 1 1] Movement Input Binding
  (Class|TankMovementComponent|IntendTurnRight (Variables|Default|GetTankMovement) AxisValue))

(event Input|AxisEvents|InputAxisMoveBackward
  (params (AxisValue :type Float%20%28single-precision%29))
  ;[1 1 1] Movement Input Binding
  (Class|TankMovementComponent|IntendMoveForward (Variables|Default|GetTankMovement) AxisValue))

(event Input|AxisEvents|InputAxisMoveForward
  (params (AxisValue :type Float%20%28single-precision%29))
  ;[1 1 1] Movement Input Binding
  (Class|TankMovementComponent|IntendMoveForward (Variables|Default|GetTankMovement) AxisValue))

(event Input|AxisEvents|InputAxisTurnLeft
  (params (AxisValue :type Float%20%28single-precision%29))
  ;[1 1 1] Movement Input Binding
  (Class|TankMovementComponent|IntendTurnRight (Variables|Default|GetTankMovement) AxisValue))

(fn ConstructionScript
  (Components|StaticMesh|SetStaticMesh (Variables|Default|Getturret) "/Game/tank/tank_fbx_Turret.tank_fbx_Turret")
  (Components|StaticMesh|SetStaticMesh (Variables|Default|GetBarrel) "/Game/tank/tank_fbx_Barrel.tank_fbx_Barrel")
  (Components|StaticMesh|SetStaticMesh (Variables|Default|GetTankTrackLeft) "/Game/tank/tank_fbx_Track.tank_fbx_Track")
  (Components|StaticMesh|SetStaticMesh (Variables|Default|GetTankTrackRight) "/Game/tank/tank_fbx_Track.tank_fbx_Track")
  (Class|PrimitiveComponent|SetNotifyRigidBodyCollision (Variables|Default|GetTankTrackLeft) true)
  (Class|PrimitiveComponent|SetNotifyRigidBodyCollision (Variables|Default|GetTankTrackRight) true))